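; Player-drivable tank Blueprint that moves, aims its camera, fires and carries a health bar widget.
; On BeginPlay it hands the barrel and turret to TankAiming, both tracks to TankMovement, and itself to the HealthBar widget.
; Input forwards throttle and turn intent to TankMovement and fire to TankAiming.
; Look axes rotate an azimuth gimbal and spring arm separately, scaled by delta time, and SwapCam toggles first- and third-person cameras.
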(event `self.ReceiveBeginPlay`
  (`TankAimingComponent.Initialize` (`self.TankAiming`) (`self.TankBarrel`) (`self.TankTurret`))
  (`TankMovementComponent.Initialise` (`self.TankMovement`) (`self.LeftTrack `) (`self.RighTrack`))
  (`self.HealthBarInitializ`))

(event `InputAxis|Move Forward`
  (params (AxisValue :type "Float (single-precision)"))
  ;[1 1 1] Throttle
  (`TankMovementComponent.IntendMoveForward` (`self.TankMovement`) AxisValue))

(event `InputAxis|AimAzimuth`
  (params (AxisValue :type "Float (single-precision)"))
  ;[1 1 1] Camera
  (`SceneComponent.K2_AddLocalRotation` (`self.Azimuth Gimbal`) (`KismetMathLibrary.MakeRotator` 0.0 0.0 (* AxisValue (`GameplayStatics.GetWorldDeltaSeconds`) 100.0)) false false))

(event `InputAxis|AimElevation`
  (params (AxisValue :type "Float (single-precision)"))
  ;[1 1 1] Camera
  (`SceneComponent.K2_AddLocalRotation` (`self.SpringArm`) (`KismetMathLibrary.MakeRotator` 0.0 (* AxisValue (`GameplayStatics.GetWorldDeltaSeconds`) 100.0)) false false))

(event `InputAxis|Move Right`
  (params (AxisValue :type "Float (single-precision)"))
  ;[1 1 1] Throttle
  (`TankMovementComponent.IntendTurnRight` (`self.TankMovement`) AxisValue))

(event `InputAction|SwapCam`
  (params (Key :type "Key Structure"))
  ;[1 1 1] Swap Camera
  (:`Pressed`
    (`ActorComponent.ToggleActive` (`self.FirstPerson`))
    (`ActorComponent.ToggleActive` (`self.ThirdPerson`))))

(event `InputAction|Fire`
  (params (Key :type "Key Structure"))
  ;[1 1 1] Fire
  (:`Pressed`
    (`TankAimingComponent.Fire` (`self.TankAiming`))))

(fn `HealthBarInitializ`
  (bind _ashealth_bar (cast `/Game/UI/HealthBar` (`WidgetComponent.GetUserWidgetObject` (`self.Widget`))))
  (set `/Game/UI/HealthBar.MyTank` self _ashealth_bar)
  (return))

(fn `UserConstructionScript`)